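; Blueprint function library for the building system that gives lookup access to buildable definitions stored in DT_BuildableDefinitions.
; One function uses a gameplay tag's name as the row name to fetch that buildable's data with a found flag.
; The other walks every row and gathers each definition's Tag field into a gameplay tag container of all buildables.
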(fn `FL_GetAllBuildableTags`
  (returns (BuildableTags1 :type "GameplayTagContainer Structure"))
  (locals (BuildableTags :type "GameplayTagContainer Structure"))
  (bind _outrownames (`DataTableFunctionLibrary.GetDataTableRowNames` "/Game/Core/Data/Tables/DT_BuildableDefinitions.DT_BuildableDefinitions"))
  (for _array_element _outrownames
    (bind _returnvalue (`|GetDataTableRow` "/Game/Core/Data/Tables/DT_BuildableDefinitions.DT_BuildableDefinitions" _array_element)
      (:`then`
        (`BlueprintGameplayTagLibrary.AddGameplayTag` (`local.BuildableTags`) (`.Tag_7_4A5738CE43F44A6BC6B9589BB2A47C00` (break `/Game/Core/Data/Structures/S_BuildableData` _returnvalue))))))
  (return (`local.BuildableTags`)))

(fn `FL_GetBuildableDataByTag`
  (params (Tag :type "GameplayTag Structure"))
  (returns (`IsFound?` :type Boolean) (BuildableData :type "/Game/Core/Data/Structures/S_BuildableData Structure"))
  (bind _returnvalue (`|GetDataTableRow` "/Game/Core/Data/Tables/DT_BuildableDefinitions.DT_BuildableDefinitions" (`BlueprintGameplayTagLibrary.GetTagName` Tag))
    (:`then`
      (return true _returnvalue))))