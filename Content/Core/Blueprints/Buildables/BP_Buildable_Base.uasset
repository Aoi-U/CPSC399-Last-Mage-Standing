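; Base actor for player-built structures, with health, a level-up system and a stats widget.
; Construction looks up mesh by buildable tag; damage lowers health and destroys the actor below zero.
; Level-up checks the player's held resources against required costs, consumes them, raises max health and refills it.
; A short timer hides the stats widget, which shows name, level and resource affordability; socket and box interface functions are empty stubs.
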(event `self.ReceiveBeginPlay`
  (bind _asw_structure_stats (cast `/Game/TopDown/Blueprints/Widgets/W_StructureStats` (`WidgetComponent.GetWidget` (`self.Widget`))))
  (`/Game/TopDown/Blueprints/Widgets/W_StructureStats.BindHealthBar` _asw_structure_stats self)
  (add `/Game/TopDown/Blueprints/Widgets/W_StructureStats.StructureLevelUp_Dispatch` _asw_structure_stats (delegate `Event StructureLevelUp`))
  (add `self.OnTakeAnyDamage` (delegate `OnTakeAnyDamage_Event`)))

(event `OnTakeAnyDamage_Event` :!signature `self.OnTakeAnyDamage`
  (params (DamagedActor :type "Actor Object Reference") (Damage :type "Float (single-precision)") (DamageType :type "DamageType Object Reference") (InstigatedBy :type "Controller Object Reference") (DamageCauser :type "Actor Object Reference"))
  (`self.F_DamageWall` Damage))

(event `Event StructureLevelUp`
  (bind _asbp_top_down_character (cast `/Game/TopDown/Blueprints/BP_TopDownCharacter` (`GameplayStatics.GetPlayerCharacter` 0)))
  (set `self.LocalHasEnoughResourceToLevelUp` true)
  ; Check if player has enough resources to level up
  (bind (_keypin _valuepin) (`|MapForEach` (`self.LevelUpRequiredResources`))
    (:`then`
      (if (< (`BlueprintMapLibrary.Map_Find` (`/Game/TopDown/Blueprints/BP_TopDownCharacter.HeldResources` _asbp_top_down_character) _keypin) _valuepin)
        (`KismetSystemLibrary.PrintString` "Not enough resources to level up!")
        (set `self.LocalHasEnoughResourceToLevelUp` false)))
    (:`CompletedPin`
      ; Level up structure and consume required materials
      (if (`self.LocalHasEnoughResourceToLevelUp`)
        (`self.F_LevelUp`)
        (message `/Game/Core/Blueprints/Interfaces/BPI_Character.IF_ConsumeResources` (`GameplayStatics.GetPlayerCharacter` 0) (`self.LevelUpRequiredResources`))
        (`KismetSystemLibrary.PrintString` "Structure leveled up successfully")
        (`self.F_UpdateStatsWidget`)))))

(event `ActivateStatsWidget`
  ; Enable strucuture stats widget for x seconds
  (bind _returnvalue (`KismetSystemLibrary.K2_SetTimerDelegate` (delegate `DeactivateStatsWidget`) 0.2))
  (set `self.StatsWidgetTimerHandle` _returnvalue)
  (`SceneComponent.SetVisibility` (`self.Widget`) true false)
  (`self.F_UpdateStatsWidget`))

(event `DeactivateStatsWidget`
  ; Enable strucuture stats widget for x seconds
  (`SceneComponent.SetVisibility` (`self.Widget`) false false))

(fn `F_CheckDeath`
  ; Destroy the structure if it is out of health
  (if (< (`self.Health`) 0.0)
    (`self.K2_DestroyActor`)))

(fn `F_DamageWall`
  (params (DamageTaken :type "Float (double-precision)"))
  ; Damage the structure by the input amount
  (set `self.Health` (- (`self.Health`) DamageTaken))
  (`self.F_CheckDeath`))

(fn `F_GetResourceData`
  (params (Name :type "/Game/Core/Data/Enums/E_Resources Enum" :default "NewEnumerator0"))
  (returns (ResourceData :type "/Game/Core/Data/Structures/S_ResourceData Structure"))
  (return (`/Game/Core/Blueprints/Game/BuildingSystemFL.FL_GetResourceDataByName` Name)))

(fn `F_LevelUp`
  (`/Engine/EditorBlueprintResources/StandardMacros.IncrementInt` (`self.Level`)
    (:`  `
      (bind _output_get (set `self.MaxHealth` (+ (`self.MaxHealth`) 100.0)))
      (set `self.Health` _output_get))))

(fn `F_UpdateStatsWidget`
  (locals (ResourceValues :type "Array of /Game/TopDown/Blueprints/OBJ_StructureStatObject Object Reference"))
  ; Update the widget corresponding to this structure
  (bind _asw_structure_stats (cast `/Game/TopDown/Blueprints/Widgets/W_StructureStats` (`WidgetComponent.GetUserWidgetObject` (`self.Widget`))))
  (bind _asbp_top_down_character (cast `/Game/TopDown/Blueprints/BP_TopDownCharacter` (`GameplayStatics.GetPlayerCharacter` 0)))
  ;; Construct the array of resource requirements
  (bind (_keypin _valuepin) (`|MapForEach` (`self.LevelUpRequiredResources`))
    (:`then`
      (bind (_resourcedata_name _resourcedata_mesh _resourcedata_image) (break `/Game/Core/Data/Structures/S_ResourceData` (`self.F_GetResourceData` _keypin)))
      (bind _returnvalue (`|GenericCreateObject` "/Game/TopDown/Blueprints/OBJ_StructureStatObject.OBJ_StructureStatObject_C" (`|GenericToText` _resourcedata_name) _resourcedata_image (not (< (`BlueprintMapLibrary.Map_Find` (`/Game/TopDown/Blueprints/BP_TopDownCharacter.HeldResources` _asbp_top_down_character) _keypin) _valuepin)) _valuepin))
      (`KismetArrayLibrary.Array_Add` (`local.ResourceValues`) _returnvalue))
    (:`CompletedPin`
      (`/Game/TopDown/Blueprints/Widgets/W_StructureStats.UpdateResourceValues` _asw_structure_stats (`.Name_51_45E0E46245240C61D94F3F8B411C0529` (break `/Game/Core/Data/Structures/S_BuildableData` (`.BuildableData` (`/Game/Core/Blueprints/Game/BuildingSystemFL.FL_GetBuildableDataByTag` (`self.BuildableTag`))))) (`local.ResourceValues`) (`self.Level`)))))

(fn `IF_GetBuildableTag`
  (returns (Tag :type "GameplayTag Structure"))
  (return (`self.BuildableTag`)))

(fn `IF_GetSockets`
  (returns (SocketComponents :type "Array of PrimitiveComponent Object Reference"))
  (return))

(fn `IF_ReturnAttackTowerBoxes`
  (returns (Boxes :type "Array of BoxComponent Object Reference"))
  (return))

(fn `IF_ReturnDefenseBoxes`
  (returns (Boxes :type "Array of BoxComponent Object Reference"))
  (return))

(fn `IF_ReturnTowerBoxes`
  (returns (Boxes :type "Array of BoxComponent Object Reference"))
  (return))

(fn `UserConstructionScript`
  (bind (_isfound_ _buildabledata) (`/Game/Core/Blueprints/Game/BuildingSystemFL.FL_GetBuildableDataByTag` (`self.BuildableTag`)))
  (`|ExecutionSequence`
    (:`then_0`
      (if _isfound_
        (`StaticMeshComponent.SetStaticMesh` (`self.BuildableMesh`) (`.Mesh_15_483FE3C44B53615959A3968EA7D062CB` (break `/Game/Core/Data/Structures/S_BuildableData` _buildabledata)))))
    (:`then_1`
      (set `self.Health` (`self.MaxHealth`)))
    (:`then_2`
      (`SceneComponent.SetWorldScale3D` (`self.BuildableMesh`) (`self.DefaultScale`)))))