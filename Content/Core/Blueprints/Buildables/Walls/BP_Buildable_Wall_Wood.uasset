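; Wooden wall buildable Blueprint that supplies its attachment or placement boxes through interface functions.
; One interface function returns six DefenseBox components and another returns two TowerBox components.
; BeginPlay and the construction script only call their parent versions, so the rest of its behavior comes from the parent class.
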(event `self.ReceiveBeginPlay`
  (`parent.ReceiveBeginPlay`))

(fn `IF_ReturnDefenseBoxes`
  (returns (Boxes :type "Array of BoxComponent Object Reference"))
  (return (`|MakeArray` (`self.DefenseBox`) (`self.DefenseBox1`) (`self.DefenseBox2`) (`self.DefenseBox3`) (`self.DefenseBox4`) (`self.DefenseBox5`))))

(fn `IF_ReturnTowerBoxes`
  (returns (Boxes :type "Array of BoxComponent Object Reference"))
  (return (`|MakeArray` (`self.TowerBox`) (`self.TowerBox1`))))

(fn `UserConstructionScript`
  (`parent.UserConstructionScript`))