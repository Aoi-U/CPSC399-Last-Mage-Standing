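; Base actor for a dropped resource pickup that the top-down player character collects by overlap.
; Construction looks up the mesh from resource data by the resource's enum name and enables physics on it.
; FInit stores the count and feeds name and count to the drop widget through a data object.
; Collection sphere overlap waits a tick, adds the resource to the character, signals an inventory update and destroys the actor.
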(event `self.ReceiveBeginPlay`)

(event `self.CollectionSphere.OnComponentBeginOverlap`
  (params (OverlappedComponent :type "PrimitiveComponent Object Reference") (OtherActor :type "Actor Object Reference") (OtherComp :type "PrimitiveComponent Object Reference") (OtherBodyIndex :type Integer) (bFromSweep :type Boolean) (SweepResult :type "HitResult Structure (by ref)"))
  ; Player pickup resource
  (`KismetSystemLibrary.DelayUntilNextTick`)
  (bind _asbp_top_down_character (cast `/Game/TopDown/Blueprints/BP_TopDownCharacter` OtherActor))
  (`/Game/TopDown/Blueprints/BP_TopDownCharacter.F_PickUpResources` _asbp_top_down_character (`self.Name`) (`self.Count`))
  (`/Game/TopDown/Blueprints/BP_TopDownCharacter.InventoryUpdated` _asbp_top_down_character)
  (`self.K2_DestroyActor`))

(fn `F_Init`
  (params (Count :type Integer))
  (`self.F_SetCount` Count)
  (`self.F_SetWidget`))

(fn `F_SetCount`
  (params (Count :type Integer))
  ; Set the count variable
  (set `self.Count` Count))

(fn `F_SetWidget`
  (bind _asw_resource_drop (cast `/Game/TopDown/Blueprints/Widgets/W_ResourceDrop` (`WidgetComponent.GetUserWidgetObject` (`self.Widget`))))
  (bind _returnvalue (`|GenericCreateObject` "/Game/TopDown/Blueprints/OBJ_ResourceDropObject.OBJ_ResourceDropObject_C" (`KismetTextLibrary.Conv_StringToText` (`|GetEnumeratorNameAsString` (`self.Name`))) (`self.Count`)))
  (`/Game/TopDown/Blueprints/Widgets/W_ResourceDrop.InitResourceValues` _asw_resource_drop _returnvalue))

(fn `UserConstructionScript`
  (`StaticMeshComponent.SetStaticMesh` (`self.ResourceMesh`) (`.Mesh_2_78ADC4F7447CBF6A8DBAFE876A27D2A7` (break `/Game/Core/Data/Structures/S_ResourceData` (`/Game/Core/Blueprints/Game/BuildingSystemFL.FL_GetResourceDataByName` (`self.Name`)))))
  (`PrimitiveComponent.SetSimulatePhysics` (`self.ResourceMesh`) true))