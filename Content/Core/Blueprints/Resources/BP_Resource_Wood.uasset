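; Wood resource actor that merges with other wood resources in range to form a single stack.
; When its CollectionSphere overlaps another BP_Resource_Wood not already being absorbed, it flags that actor, adds its Count to its own, refreshes the widget and destroys it.
; The IsBeingAbsorbed flag guards against absorbing the same pile more than once.
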(event `self.CollectionSphere.OnComponentBeginOverlap`
  (params (OverlappedComponent :type "PrimitiveComponent Object Reference") (OtherActor :type "Actor Object Reference") (OtherComp :type "PrimitiveComponent Object Reference") (OtherBodyIndex :type Integer) (bFromSweep :type Boolean) (SweepResult :type "HitResult Structure (by ref)"))
  ; Stack wood resources together if within range
  (if (!= OtherActor self)
    (bind _asbp_resource_wood (cast `/Game/Core/Blueprints/Resources/BP_Resource_Wood` OtherActor))
    (if (not (`/Game/Core/Blueprints/Resources/BP_Resource_Base.IsBeingAbsorbed` _asbp_resource_wood))
      (set `/Game/Core/Blueprints/Resources/BP_Resource_Base.IsBeingAbsorbed` true _asbp_resource_wood)
      (set `self.Count` (+ (`self.Count`) (`/Game/Core/Blueprints/Resources/BP_Resource_Base.Count` _asbp_resource_wood)))
      (`self.F_SetWidget`)
      (`self.K2_DestroyActor` _asbp_resource_wood))))

(fn `UserConstructionScript`
  (`parent.UserConstructionScript`))