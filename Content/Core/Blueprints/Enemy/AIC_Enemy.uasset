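; AIC_Enemy is the AI controller for enemies derived from BP_Enemy_Base.
; On possess, it seeds the BB_Enemy blackboard with the pawn's enemy type, spawn position as home, and attack range as target range, then runs BT_EnemyAI.
; The beacon location comes from a BP_BeaconTest actor found in the level, which a comment marks as a temporary stand-in.
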(event `self.ReceiveBeginPlay`)

(event `self.ReceivePossess`
  (params (PossessedPawn :type "Pawn Object Reference"))
  (bind _asbp_enemy_base (cast `/Game/Core/Blueprints/Enemy/BP_Enemy_Base` PossessedPawn))
  ; Change beacon test later
  (bind _blackboardcomponent (`self.UseBlackboard` "/Game/Core/Blueprints/Enemy/BB_Enemy.BB_Enemy"))
  (`BlackboardComponent.SetValueAsEnum` _blackboardcomponent "EnemyType" (`/Game/Core/Blueprints/Enemy/BP_Enemy_Base.Enemy Type` _asbp_enemy_base))
  (bind _returnvalue (`GameplayStatics.GetActorOfClass` "/Game/Core/Blueprints/Enemy/BP_BeaconTest.BP_BeaconTest_C"))
  (`BlackboardComponent.SetValueAsVector` _blackboardcomponent "BeaconLocation" (`self.K2_GetActorLocation` _returnvalue))
  (`BlackboardComponent.SetValueAsVector` _blackboardcomponent "HomeLocation" (`self.K2_GetActorLocation` _asbp_enemy_base))
  (`BlackboardComponent.SetValueAsFloat` _blackboardcomponent "TargetRange" (`/Game/Core/Blueprints/Enemy/BP_Enemy_Base.AttackRange` _asbp_enemy_base))
  (`self.RunBehaviorTree` "/Game/Core/Blueprints/Enemy/BT_EnemyAI.BT_EnemyAI"))

(fn `UserConstructionScript`)