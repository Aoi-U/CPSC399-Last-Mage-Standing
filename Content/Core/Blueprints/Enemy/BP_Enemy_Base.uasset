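; Base enemy actor that detects players and Obstacle-tagged structures, takes damage and drops resources on death.
; Proximity and attack spheres write target, aggro and in-range state to the AI controller's Blackboard.
; When the target leaves attack range, it scans for a replacement, but the following reset clears target and focus regardless.
; Damage from Obstacle-tagged causers is ignored entirely; other hits flash the material and reduce health.
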(event `self.ReceiveBeginPlay`
  (set `self.CurrentHealth` (`self.MaxHealth`))
  ; Set initial values
  (set `CharacterMovementComponent.MaxWalkSpeed` (`self.MovementSpeed`) (`self.CharacterMovement`))
  (set `self.OriginalMaterial` (`PrimitiveComponent.GetMaterial` (`self.Mesh`) 0))
  (`BlackboardComponent.SetValueAsFloat` (`AIBlueprintHelperLibrary.GetBlackboard` (`AIBlueprintHelperLibrary.GetAIController` self)) "TargetRange" (`self.AttackRange`))
  (set `self.CurrentTarget` null)
  (bind _output_get (set `self.IsAggroed` false))
  (`BlackboardComponent.SetValueAsBool` (`AIBlueprintHelperLibrary.GetBlackboard` (`AIBlueprintHelperLibrary.GetAIController` self)) "IsAggroed" _output_get))

(event `self.ReceiveTick`
  (params (DeltaSeconds :type "Float (single-precision)")))

(event `self.ReceiveAnyDamage`
  (params (Damage :type "Float (single-precision)") (DamageType :type "DamageType Object Reference") (InstigatedBy :type "Controller Object Reference") (DamageCauser :type "Actor Object Reference"))
  ; Ignore Aggro if tower hits enemy
  (if (not (`self.ActorHasTag` DamageCauser "Obstacle"))
    ; Check if health < 0
    (set `self.CurrentTarget` DamageCauser)
    (`KismetSystemLibrary.PrintString` "Enemy Took Damage")
    (set `self.CurrentHealth` (- (`self.CurrentHealth`) Damage))
    ;; Go white on hit
    (`PrimitiveComponent.SetMaterial` (`self.Mesh`) 0 "/Game/Core/Blueprints/Enemy/M_HitFlash.M_HitFlash")
    (`KismetSystemLibrary.Delay` 0.1)
    (`PrimitiveComponent.SetMaterial` (`self.Mesh`) 0 (`self.OriginalMaterial`))
    (if (<= (`self.CurrentHealth`) 0.0)
      ; Kill enemy
      (`KismetSystemLibrary.PrintString` "Death")
      (`/Game/Core/Components/ResourceManagerComponent.F_DropResource` (`self.ResourceManagerComponent`) (`self.Resource`) (`KismetMathLibrary.RandomIntegerInRange` (`self.MinDropCount`) (`self.MaxDropCount`)) (`self.GetTransform`))
      (`self.K2_DestroyActor`))))

(event `self.ProximitySensor.OnComponentBeginOverlap`
  (params (OverlappedComponent :type "PrimitiveComponent Object Reference") (OtherActor :type "Actor Object Reference") (OtherComp :type "PrimitiveComponent Object Reference") (OtherBodyIndex :type Integer) (bFromSweep :type Boolean) (SweepResult :type "HitResult Structure (by ref)"))
  (bind _returnvalue (`AIBlueprintHelperLibrary.GetBlackboard` (`AIBlueprintHelperLibrary.GetAIController` self)))
  ; Initial Validity Check
  (`/Engine/EditorBlueprintResources/StandardMacros.IsValid` (`BlackboardComponent.GetValueAsObject` (`AIBlueprintHelperLibrary.GetBlackboard` (`AIBlueprintHelperLibrary.GetAIController` self)) "TargetActor")
    (:`Is Not Valid`
      (for _array_element (`PrimitiveComponent.GetOverlappingActors` (`self.ProximitySensor`) "/Script/Engine.Actor")
        ; Check for valid objects within sensor
        (bind _asbp_top_down_character (cast `/Game/TopDown/Blueprints/BP_TopDownCharacter` _array_element)
          (:`then`
            ; Set values when conditions are true
            (`BlackboardComponent.SetValueAsObject` _returnvalue "TargetActor" _asbp_top_down_character)
            (`KismetSystemLibrary.PrintString` "Player Detected")
            (bind _output_get (set `self.IsAggroed` true))
            (`BlackboardComponent.SetValueAsBool` _returnvalue "IsAggroed" _output_get)
            (break))
          (:`CastFailed`
            (if (`self.ActorHasTag` _array_element "Obstacle")
              (`KismetSystemLibrary.PrintString` "Structure Detected")
              (`BlackboardComponent.SetValueAsObject` _returnvalue "TargetActor" _array_element)
              (bind _output_get_2 (set `self.IsAggroed` true))
              (`BlackboardComponent.SetValueAsBool` _returnvalue "IsAggroed" _output_get_2))))))))

(event `self.AttackSphere.OnComponentBeginOverlap`
  (params (OverlappedComponent :type "PrimitiveComponent Object Reference") (OtherActor :type "Actor Object Reference") (OtherComp :type "PrimitiveComponent Object Reference") (OtherBodyIndex :type Integer) (bFromSweep :type Boolean) (SweepResult :type "HitResult Structure (by ref)"))
  (bind _returnvalue (`AIBlueprintHelperLibrary.GetBlackboard` (`AIBlueprintHelperLibrary.GetAIController` self)))
  (bind _returnvalue_2 (`AIBlueprintHelperLibrary.GetBlackboard` (`AIBlueprintHelperLibrary.GetAIController` self)))
  (bind _returnvalue_3 (`BlackboardComponent.GetValueAsObject` _returnvalue "TargetActor"))
  ; Initial checking
  (`KismetSystemLibrary.PrintString` "Is In Range")
  (`/Engine/EditorBlueprintResources/StandardMacros.IsValid` _returnvalue_3
    (:`Is Valid`
      (if (== OtherActor _returnvalue_3)
        (`BlackboardComponent.SetValueAsBool` _returnvalue "IsInRange" true)))
    (:`Is Not Valid`
      ; Set up values
      (bind _asbp_top_down_character (cast `/Game/TopDown/Blueprints/BP_TopDownCharacter` OtherActor)
        (:`then`
          (`BlackboardComponent.SetValueAsObject` _returnvalue_2 "TargetActor" _asbp_top_down_character)
          (`BlackboardComponent.SetValueAsBool` _returnvalue_2 "IsInRange" true :!label _label)
          (bind _output_get (set `self.IsAggroed` true))
          (`BlackboardComponent.SetValueAsBool` _returnvalue_2 "IsAggroed" _output_get))
        (:`CastFailed`
          (if (`self.ActorHasTag` OtherActor "Obstacle")
            (`BlackboardComponent.SetValueAsObject` _returnvalue_2 "TargetActor" OtherActor)
            (goto _label)))))))

(event `self.AttackSphere.OnComponentEndOverlap`
  (params (OverlappedComponent :type "PrimitiveComponent Object Reference") (OtherActor :type "Actor Object Reference") (OtherComp :type "PrimitiveComponent Object Reference") (OtherBodyIndex :type Integer))
  (bind _returnvalue (`AIBlueprintHelperLibrary.GetAIController` self))
  (bind _returnvalue_2 (`AIBlueprintHelperLibrary.GetBlackboard` (`AIBlueprintHelperLibrary.GetAIController` self)))
  (bind _returnvalue_3 (`AIBlueprintHelperLibrary.GetBlackboard` _returnvalue))
  ; Initial Checking
  ;; When something exists, run check to get valid values
  (if (== OtherActor (`BlackboardComponent.GetValueAsObject` (`AIBlueprintHelperLibrary.GetBlackboard` (`AIBlueprintHelperLibrary.GetAIController` self)) "TargetActor"))
    (for _array_element (`PrimitiveComponent.GetOverlappingActors` (`self.AttackSphere`) "/Script/Engine.Actor")
      ; As long as the enemy exists, you can set the aggro
      (bind _asbp_top_down_character (cast `/Game/TopDown/Blueprints/BP_TopDownCharacter` _array_element)
        (:`then`
          (`BlackboardComponent.SetValueAsObject` _returnvalue_2 "TargetActor" _asbp_top_down_character)
          (bind _output_get (set `self.IsAggroed` true :!label _label_2))
          (`BlackboardComponent.SetValueAsBool` _returnvalue_2 "IsAggroed" _output_get)
          (`BlackboardComponent.SetValueAsBool` _returnvalue_2 "IsInRange" true)
          (`KismetSystemLibrary.PrintString` "New Target Set")
          (break))
        (:`CastFailed`
          (if (`self.ActorHasTag` _array_element "Obstacle")
            (`BlackboardComponent.SetValueAsObject` _returnvalue_2 "TargetActor" _array_element)
            (goto _label_2)))))
    ; Reset values when there is nothing to track
    (`BlackboardComponent.SetValueAsBool` _returnvalue_3 "IsInRange" false)
    (`BlackboardComponent.SetValueAsObject` _returnvalue_3 "TargetActor" null)
    (bind _output_get_2 (set `self.IsAggroed` false))
    (`BlackboardComponent.SetValueAsBool` _returnvalue_3 "IsAggroed" _output_get_2)
    (`AIController.K2_ClearFocus` _returnvalue)))

(fn `UserConstructionScript`)