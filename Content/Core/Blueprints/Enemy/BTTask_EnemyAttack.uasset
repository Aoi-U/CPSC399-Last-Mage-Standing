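; Behavior tree task that makes a BP_Enemy_Base pawn perform an attack on the blackboard target actor.
; It plays the enemy's attack montage, waits out its returned length, then applies the enemy's damage with debug prints before finishing successfully.
; The AttackRange check compares the pawn's location with its own rather than the target's, so target distance is never tested.
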(event `self.ReceiveExecuteAI`
  (params (OwnerController :type "AIController Object Reference") (ControlledPawn :type "Pawn Object Reference"))
  (bind _asbp_enemy_base (cast `/Game/Core/Blueprints/Enemy/BP_Enemy_Base` ControlledPawn)
    (:`then`
      (bind _returnvalue (`Character.PlayAnimMontage` _asbp_enemy_base (`/Game/Core/Blueprints/Enemy/BP_Enemy_Base.MyAttackAnimation` _asbp_enemy_base) 1.0 "None")) ; Change this for later
      (`KismetSystemLibrary.Delay` _returnvalue)
      (`KismetSystemLibrary.PrintString` "Attack")
      (if (< (`KismetMathLibrary.Vector_Distance` (`Actor.K2_GetActorLocation` ControlledPawn) (`Actor.K2_GetActorLocation` _asbp_enemy_base)) (`/Game/Core/Blueprints/Enemy/BP_Enemy_Base.AttackRange` _asbp_enemy_base))
        (bind _damage (`/Game/Core/Blueprints/Enemy/BP_Enemy_Base.Damage` _asbp_enemy_base))
        (`GameplayStatics.ApplyDamage` (`BTFunctionLibrary.GetBlackboardValueAsActor` (`self.BlackboardKey_TargetActor`)) _damage OwnerController ControlledPawn)
        (`KismetSystemLibrary.PrintString` (`KismetStringLibrary.Conv_DoubleToString` _damage))))
    (:`CastFailed`
      _))
  (`self.FinishExecute` true))