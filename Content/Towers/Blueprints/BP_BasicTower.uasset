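; Basic tower actor that periodically fires at its current target.
; A looping timer set on BeginPlay runs Targeting, which passes the target's location to the ABP_BasicTracking anim instance for tracking.
; When the target is valid, it also spawns an actor above the tower, handing it damage and the target, and plays a 2D fire sound.
; Target selection happens outside these graphs.
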(event `self.ReceiveBeginPlay`
  (`parent.ReceiveBeginPlay`)
  (`KismetSystemLibrary.K2_SetTimer` null "Targeting" 0.4 true))

(fn `Targeting`
  (bind _asabp_basic_tracking (cast `/Game/Towers/Animations/ABP_BasicTracking` (`SkeletalMeshComponent.GetAnimInstance` (`self.Mesh`))))
  (if (`KismetSystemLibrary.IsValid` (`self.CurrentTarget`))
    (set `/Game/Towers/Animations/ABP_BasicTracking.TargetLocation` (`self.K2_GetActorLocation` (`self.CurrentTarget`)) _asabp_basic_tracking)
    (`|SpawnActorFromClass` "/Game/Towers/Blueprints/BP_FireProjectile.BP_FireProjectile_C" (`KismetMathLibrary.Conv_VectorToTransform` (+ (`self.K2_GetActorLocation`) (0.0 0.0 300.0))) "Undefined" "MultiplyWithRoot" null (`self.Damage`) (`self.CurrentTarget`) null)
    (`GameplayStatics.PlaySound2D` "/Game/Towers/Sounds/fireshootsound.fireshootsound" 1.0 1.0 0.0 null null)))

(fn `UserConstructionScript`
  (`parent.UserConstructionScript`))