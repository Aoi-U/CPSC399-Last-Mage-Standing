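; BP_ProjectileMaster is a tower projectile that homes in on a target enemy and damages it on overlap.
; InitProjectile stores the target and damage and points the ProjectileMovement homing component at the target's root; the construction script also sets that homing target.
; Overlapping any BP_Enemy_Base actor applies the stored damage and destroys the projectile.
; A lifespan set on BeginPlay removes projectiles that never hit.
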(event `self.ReceiveBeginPlay`
  (`self.SetLifeSpan` 5.0))

(event `self.ReceiveActorBeginOverlap`
  (params (OtherActor :type "Actor Object Reference"))
  (bind _asbp_enemy_base (cast `/Game/Core/Blueprints/Enemy/BP_Enemy_Base` OtherActor))
  (`GameplayStatics.ApplyDamage` _asbp_enemy_base (`self.Damage`) null self)
  (`self.K2_DestroyActor`))

(fn `InitProjectile`
  (params (Target :type "Actor Object Reference") (DamageAmount :type "Float (double-precision)"))
  (set `self.TargetActor` Target)
  (set `self.Damage` DamageAmount)
  (set `ProjectileMovementComponent.HomingTargetComponent` (`Actor.RootComponent` Target) (`self.ProjectileMovement`)))

(fn `UserConstructionScript`
  (set `ProjectileMovementComponent.HomingTargetComponent` (`Actor.RootComponent` (`self.TargetActor`)) (`self.ProjectileMovement`)))