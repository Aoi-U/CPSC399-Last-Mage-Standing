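; BP_TowerMaster is a tower Blueprint that handles enemy detection and target selection, with no firing logic of its own.
; The construction script sizes the Sphere component to AttackRange and hides BuildableMesh.
; Actor overlap events add and remove BP_Enemy_Base actors in EnemiesInRange without using Tick.
; An entering enemy becomes CurrentTarget if none is valid; when the target leaves, the first remaining enemy takes over, or it clears.
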(event `self.ReceiveBeginPlay`
  (`parent.ReceiveBeginPlay`))

(event `self.ReceiveActorBeginOverlap`
  (params (OtherActor :type "Actor Object Reference"))
  (`parent.ReceiveActorBeginOverlap` OtherActor)
  (bind _asbp_enemy_base (cast `/Game/Core/Blueprints/Enemy/BP_Enemy_Base` OtherActor))
  (`KismetArrayLibrary.Array_AddUnique` (`self.EnemiesInRange`))
  (if (not (`KismetSystemLibrary.IsValid` (`self.CurrentTarget`)))
    (set `self.CurrentTarget` _asbp_enemy_base)))

(event `self.ReceiveActorEndOverlap`
  (params (OtherActor :type "Actor Object Reference"))
  (bind _asbp_enemy_base (cast `/Game/Core/Blueprints/Enemy/BP_Enemy_Base` OtherActor))
  (`KismetArrayLibrary.Array_RemoveItem` (`self.EnemiesInRange`))
  (if (== _asbp_enemy_base (`self.CurrentTarget`))
    (if (`KismetArrayLibrary.Array_IsEmpty` (`self.EnemiesInRange`))
      (set `self.CurrentTarget` null)
      (else
        (set `self.CurrentTarget` (`|GetArrayItem` (`self.EnemiesInRange`)))))))

(fn `UserConstructionScript`
  (`parent.UserConstructionScript`)
  (`SphereComponent.SetSphereRadius` (`self.Sphere`) (`self.AttackRange`) true)
  (`SceneComponent.SetVisibility` (`self.BuildableMesh`) false false))