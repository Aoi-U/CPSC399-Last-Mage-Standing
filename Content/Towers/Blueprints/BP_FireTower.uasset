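; Fire tower that periodically launches a fire projectile at its current target.
; A looping timer started on BeginPlay runs Targeting, which passes the target's location to the ABP_targetLock anim instance for aiming.
; It then spawns BP_FireProjectile at the mesh's Palm socket and initializes it with the target and the projectile's own Damage value.
; CurrentTarget is only read here, never selected.
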(event `self.ReceiveBeginPlay`
  (`KismetSystemLibrary.K2_SetTimer` null "Targeting" 1.6 true))

(event `self.ReceiveTick`
  (params (DeltaSeconds :type "Float (single-precision)")))

(fn `Targeting`
  (bind _asabp_target_lock (cast `/Game/Towers/Blueprints/ABP_targetLock` (`SkeletalMeshComponent.GetAnimInstance` (`self.Mesh`))))
  (if (`KismetSystemLibrary.IsValid` (`self.CurrentTarget`))
    (set `/Game/Towers/Blueprints/ABP_targetLock.TargetLocation` (`self.K2_GetActorLocation` (`self.CurrentTarget`)) _asabp_target_lock)
    (bind _returnvalue (`|SpawnActorFromClass` "/Game/Towers/Blueprints/BP_FireProjectile.BP_FireProjectile_C" (`KismetMathLibrary.Conv_VectorToTransform` (`SceneComponent.GetSocketLocation` (`self.Mesh`) "Palm")) "Undefined" "MultiplyWithRoot" null null))
    (`/Game/Towers/Blueprints/BP_ProjectileMaster.InitProjectile` _returnvalue (`self.CurrentTarget`) (`/Game/Towers/Blueprints/BP_ProjectileMaster.Damage` _returnvalue))))

(fn `UserConstructionScript`
  (`parent.UserConstructionScript`))