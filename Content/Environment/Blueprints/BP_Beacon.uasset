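; BP_Beacon is a damageable beacon actor with a health bar widget, whose death ends the game.
; On BeginPlay it binds the W_BeaconHealthBar widget to itself and routes any damage it takes into FDamageWall, whose body is not shown here.
; FCheckDeath shows the game over menu and pauses the game when Health drops below zero, though no call to it appears in these graphs.
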(event `self.ReceiveBeginPlay`
  (bind _asw_beacon_health_bar (cast `/Game/TopDown/Blueprints/Widgets/W_BeaconHealthBar` (`WidgetComponent.GetWidget` (`self.HealthWidget`))))
  (`/Game/TopDown/Blueprints/Widgets/W_BeaconHealthBar.BindHealthBar` _asw_beacon_health_bar self)
  (add `Actor.OnTakeAnyDamage` (delegate `TakeDamage_Event`)))

(event `TakeDamage_Event`
  (params (DamagedActor :type "Actor Object Reference") (Damage :type "Float (single-precision)") (DamageType :type "DamageType Object Reference") (InstigatedBy :type "Controller Object Reference") (DamageCauser :type "Actor Object Reference"))
  (`self.F_DamageWall` Damage))

(fn `F_CheckDeath`
  (if (< (`self.Health`) 0.0)
    (bind _returnvalue (`|CreateWidget` "/Game/TopDown/Blueprints/Widgets/W_GameOverMenu.W_GameOverMenu_C" (`GameplayStatics.GetPlayerController` 0)))
    (`UserWidget.AddToViewport` _returnvalue 0)
    (`GameplayStatics.SetGamePaused` true)))

(fn `UserConstructionScript`)