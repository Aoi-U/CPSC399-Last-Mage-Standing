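; Destroyable environment actor, apparently the master Blueprint, that drops resources for the player when destroyed.
; Each DamageTaken event removes a fixed amount of Health; at zero it has the player character's ResourceManagerComponent drop a random count of its ResourceType nearby, then destroys itself.
; BeginPlay places the Prompt just above the mesh bounds, and player overlap toggles its visibility and the PlayerNearby flag.
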(event `DamageTaken`
  (bind _returnvalue (`KismetMathLibrary.RandomFloatInRange` 150.0 350.0))
  ; Tower takes damage at constant 25, destroy and drops resources when health below 0
  (bind _output_get (set `self.Health` (- (`self.Health`) 25.0)))
  (if (<= _output_get 0.0)
    (bind _asbp_top_down_character (cast `/Game/TopDown/Blueprints/BP_TopDownCharacter` (`GameplayStatics.GetPlayerCharacter` 0)))
    (`/Game/Core/Components/ResourceManagerComponent.F_DropResource` (`/Game/TopDown/Blueprints/BP_TopDownCharacter.ResourceManagerComponent` _asbp_top_down_character) (`self.ResourceType`) (`KismetMathLibrary.RandomIntegerInRange` 1 5) (`KismetMathLibrary.Conv_VectorToTransform` (+ (`self.K2_GetActorLocation`) (`KismetMathLibrary.MakeVector` _returnvalue _returnvalue 200.0))))
    (`self.K2_DestroyActor`)))

(event `self.ReceiveBeginPlay`
  (`SceneComponent.K2_SetRelativeLocation` (`self.Prompt`) (`KismetMathLibrary.MakeVector` 0.0 0.0 (+ (.z (`.Max` (`StaticMeshComponent.GetLocalBounds` (`self.StaticMesh`)))) 50.0)) false false))

(event `self.ReceiveActorBeginOverlap`
  (params (OtherActor :type "Actor Object Reference"))
  (cast `/Game/TopDown/Blueprints/BP_TopDownCharacter` OtherActor)
  (set `self.PlayerNearby` true)
  (`SceneComponent.SetVisibility` (`self.Prompt`) true false))

(event `self.ReceiveActorEndOverlap`
  (params (OtherActor :type "Actor Object Reference"))
  (cast `/Game/TopDown/Blueprints/BP_TopDownCharacter` OtherActor)
  (set `self.PlayerNearby` false)
  (`SceneComponent.SetVisibility` (`self.Prompt`) false false))

(fn `UserConstructionScript`)