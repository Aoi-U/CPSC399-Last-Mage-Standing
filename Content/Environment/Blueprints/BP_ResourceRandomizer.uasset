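; BP_ResourceRandomizer is an environment actor meant to scatter random tree, rock or crystal resources around itself at construction time.
; The construction script, guarded by IsConstructing, picks the class array matching ResourceType and adds SpawnCount child actor components with random classes and flat random offsets scaled up to SpawnRadius.
; Clearing and spawning are nested inside the loop destroying SpawnedActors, an array this script never fills.
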(fn `UserConstructionScript`
  (locals (ActiveClasses :type "Array of /Game/Environment/Blueprints/BP_DestroyableMaster Class Reference"))
  (bind _returnvalue (`KismetArrayLibrary.Array_Length` (`local.ActiveClasses`)))
  (if (not (`self.isConstructing`))
    (set `self.isConstructing` true)
    (for _array_element (`self.SpawnedActors`)
      (`self.K2_DestroyActor` _array_element)
      (`KismetArrayLibrary.Array_Clear` (`self.SpawnedActors`))
      (switch `/Game/Environment/Blueprints/E_ResourceType` (`self.ResourceType`)
        (:`NewEnumerator0`
          (set `local.ActiveClasses` (`self.TreeClasses`))
          (`KismetSystemLibrary.PrintString` (`KismetStringLibrary.Conv_IntToString` _returnvalue)))
        (:`NewEnumerator1`
          (set `local.ActiveClasses` (`self.RockClasses`)))
        (:`NewEnumerator2`
          (set `local.ActiveClasses` (`self.CrystalClasses`))))
      (if (> _returnvalue 0)
        (for _ (range (`self.SpawnCount`))
          (bind _returnvalue_2 (`AddComponent|NODE_AddChildActorComponent-0` :`RelativeTransform` (`KismetMathLibrary.MakeTransform` (* (`KismetMathLibrary.MakeVector` (`KismetMathLibrary.RandomFloatInRange` -1.0 1.0) (`KismetMathLibrary.RandomFloatInRange` -1.0 1.0)) (`KismetMathLibrary.RandomFloatInRange` 0.0 (`self.SpawnRadius`))))))
          (`ChildActorComponent.SetChildActorClass` _returnvalue_2 (`|GetArrayItem` (`local.ActiveClasses`) (`KismetMathLibrary.RandomIntegerInRange` 0 (`KismetArrayLibrary.Array_LastIndex` (`local.ActiveClasses`))))))
        (set `self.isConstructing` false)))))